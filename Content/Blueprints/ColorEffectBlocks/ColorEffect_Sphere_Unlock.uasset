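; Color effect block variant for a sphere unlock that plays a level sequence once its Cube is hidden.
; Tick polls an enable flag and the Cube's visibility, with a DoOnce gating the trigger.
; It creates a level sequence player that disables movement input and hides the player and HUD during playback.
; Construction defers to the parent class.
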(event EventTick
  (params (DeltaSeconds :type Float%20%28single-precision%29))
  ;[1 1 1] PlaySequence
  (if (Variables|Default|GetEnableSequence)
    (if (not (Rendering|IsVisible (Variables|Default|GetCube)))
      (Utilities|FlowControl|DoOnce false
        (:Completed
          (bind _returnvalue (Sequencer|Player|CreateLevelSequencePlayer (Variables|Default|GetSequence) (Utilities|Struct|MakeMovieSceneSequencePlaybackSettings false "(Value=0)" 1.0 0.0 false false true false true true)))
          (Sequencer|Player|Play _returnvalue :!class /Script/MovieScene.MovieSceneSequencePlayer))))))

(fn ConstructionScript
  (|CallParentFunction))