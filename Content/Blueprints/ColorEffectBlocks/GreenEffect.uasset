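; GreenEffect is a storm effect actor for the color block system that damages the first-person character when its capsule is overlapped.
; On BeginPlay it plays a sound, then a timeline lerps the storm component to a random point in a box while the laser stays hidden.
; On arrival it shows the laser, spawns a ColorEffect_Parent block at its Box component with effect flags passed through, then destroys itself.
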(event OnComponentBeginOverlap(Capsule)
  (params (OverlappedComponent :type Primitive%20Component%20Object%20Reference) (OtherActor :type Actor%20Object%20Reference) (OtherComp :type Primitive%20Component%20Object%20Reference) (OtherBodyIndex :type Integer) (bFromSweep :type Boolean) (SweepResult :type Hit%20Result%20Structure%20%28by%20ref%29))
  ;[1 1 1] Event when Player gets into Storm
  (bind _asfirst_person_character (Utilities|Casting|CastToFirstPersonCharacter OtherActor))
  (Game|Damage|ApplyDamage _asfirst_person_character 1.0 0 0))

(event EventBeginPlay
  (bind _box (Variables|Default|GetBox))
  ;[1 1 1] Set Laser Visibility false
  (Rendering|SetVisibility (Variables|Default|GetBP_ky_laser01) false false)
  ;[1 1 1] Play Sound
  (Audio|PlaySoundatLocation "/Game/Sounds/GreenColorBlock.GreenColorBlock" (Transformation|GetWorldLocation (Variables|Default|GetBox)) "0, 0, 0" 0.1 1.0 0.0 0 0 0)
  ;[1 1 1] Move to Rnd Location
  (Utilities|FlowControl|Delay 1.0)
  (Variables|Default|SetNewRndLocation (Math|Random|RandomPointinBoundingBox "0, 0, 0" "1000.000000,1000.000000,250.000000"))
  (bind _alpha (Timeline|Move PlayFromStart)
    (:Update
      (Transformation|SetRelativeLocation (Variables|Default|GetBP_ky_storm) (Math|Vector|Lerp(Vector) (Variables|Default|GetOldRndLocation) (Variables|Default|GetNewRndLocation) _alpha) false false)
      (Rendering|SetVisibility (Variables|Default|GetBP_ky_laser01) false false))
    (:Finished
      ;[1 1 1] On Arrival Activate Effect & Spawn Block & Delete BP
      (Variables|Default|SetOldRndLocation (Variables|Default|GetNewRndLocation))
      (Rendering|SetVisibility (Variables|Default|GetBP_ky_laser01) true false)
      (Utilities|FlowControl|Delay 1.0)
      (Game|SpawnActorfromClass "/Game/Blueprints/ColorEffectBlocks/ColorEffect_Parent.ColorEffect_Parent_C" (Math|Transform|MakeTransform (Transformation|GetWorldLocation _box) (Transformation|GetWorldRotation _box)) "Undefined" 0 (Variables|Default|GetR_Effect) (Variables|Default|GetB_Effect) (Variables|Default|GetG_Effect) 1.0 true false 0)
      (Utilities|FlowControl|Delay 1.0)
      (Actor|DestroyActor))))

(fn ConstructionScript)