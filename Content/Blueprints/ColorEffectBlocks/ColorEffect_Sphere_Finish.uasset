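; Finish variant of the color effect sphere blocks that triggers the game's ending.
; When its Cube component is overlapped by a ColorEffectProjectile with a ColorVal of 2, it plays the EndScene level sequence a single time.
; After a fixed delay, it opens the MainMenu level.
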(event OnComponentBeginOverlap(Cube)
  (params (OverlappedComponent :type Primitive%20Component%20Object%20Reference) (OtherActor :type Actor%20Object%20Reference) (OtherComp :type Primitive%20Component%20Object%20Reference) (OtherBodyIndex :type Integer) (bFromSweep :type Boolean) (SweepResult :type Hit%20Result%20Structure%20%28by%20ref%29))
  (bind _ascolor_effect_projectile (Utilities|Casting|CastToColorEffectProjectile OtherActor))
  (if (== (Variables|/Game/PlayerBP/Blueprints/ColorEffectProjectile.ColorEffectProjectile_C|GetColorVal _ascolor_effect_projectile) 2)
    (Utilities|FlowControl|DoOnce false
      (:Completed
        (bind _returnvalue (Sequencer|Player|CreateLevelSequencePlayer "/Game/Cinematic/EndScene.EndScene" (Utilities|Struct|MakeMovieSceneSequencePlaybackSettings false "(Value=0)")))
        (Sequencer|Player|Play _returnvalue :!class /Script/MovieScene.MovieSceneSequencePlayer)
        (Utilities|FlowControl|Delay 9.0)
        (Game|OpenLevel(byName) "MainMenu")))))

(fn ConstructionScript
  (|CallParentFunction))