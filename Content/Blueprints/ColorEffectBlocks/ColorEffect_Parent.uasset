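; Base paintable block that accumulates red, blue or green from ColorEffectProjectile hits, tinting a dynamic material.
; At full charge, enabled effects trigger: red explodes with radial damage, blue spawns a temporary BlueColorSphere, green restores nearby hidden blocks, heals the player or spawns GreenEffect actors.
; Black enemy shots reset the color and start a cooldown that absorbs projectiles.
; A detection sphere reports colored/black state changes to the player through ColorBlockNear.
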(event OnComponentBeginOverlap(Cube)
  (params (OverlappedComponent :type Primitive%20Component%20Object%20Reference) (OtherActor :type Actor%20Object%20Reference) (OtherComp :type Primitive%20Component%20Object%20Reference) (OtherBodyIndex :type Integer) (bFromSweep :type Boolean) (SweepResult :type Hit%20Result%20Structure%20%28by%20ref%29))
  (bind _cube (Variables|Default|GetCube))
  (bind _cube_2 (Variables|Default|GetCube))
  (bind _p_fire (Variables|Default|GetP_Fire))
  (bind _p_sparks (Variables|Default|GetP_Sparks))
  (bind _cube_3 (Variables|Default|GetCube))
  ;[1 1 1] Get Projectile Color Number when Hit Event
  (bind _ascolor_effect_projectile (Utilities|Casting|CastToColorEffectProjectile OtherActor))
  (Variables|Default|SetProj _ascolor_effect_projectile)
  (if (Variables|Default|GetBlackCooldown)
    (Actor|DestroyActor (Variables|Default|GetProj))
    (else
      (CallFunction|UpdateColor)
      (switch int (Variables|/Game/PlayerBP/Blueprints/ColorEffectProjectile.ColorEffectProjectile_C|GetColorVal _ascolor_effect_projectile)
        (:0
          ;[1 1 1] Limit Color Editing
          (Utilities|FlowControl|Sequence
            (:then_0
              (if (not (>= (Variables|Default|GetCountR) 1.0))
                ;[1 1 1] Counting Collisions / Adding Color
                (bind _output_get (Variables|Default|SetCountR (+ (Variables|Default|GetCountR) 0.1)))
                (Rendering|Material|SetVectorParameterValue (Variables|Default|GetDynamic%20Material) "BaseColor" (Math|Color|MakeColor _output_get 0.0 0.0) :!class /Script/Engine.MaterialInstanceDynamic)))
            (:then_1
              ;[1 1 1] Graphic Visibility (Effect)
              (Rendering|SetVisibility _p_fire true false)
              (Rendering|SetVisibility _p_sparks false false)
              ;[1 1 1] Destroy Projectile
              (Actor|DestroyActor (Variables|Default|GetProj))
              ;[1 1 1] Check if Block has Active
              (if (Variables|ColorEffectsVar|GetActivRedEffect)
                ;[1 1 1] Red Color Effect | Destroy Block & Deal Damage
                (if (>= (Variables|Default|GetCountR) 1.0)
                  (Components|Activation|Activate (Variables|Default|GetP_Explosion) false)
                  (Utilities|FlowControl|Delay 0.2)
                  (Rendering|SetVisibility _cube false false)
                  (Collision|SetCollisionEnabled _cube "NoCollision")
                  (Rendering|SetVisibility (Variables|Default|GetP_Fire) false false)
                  (Variables|Default|SetHasColor false)
                  ;[1 1 1] Radial Damage
                  (Game|Damage|ApplyRadialDamage (Variables|RedColorEffect|GetDamage) (Transformation|GetWorldLocation (Variables|Default|GetCube)) (Variables|RedColorEffect|GetDamageRadius) 0 0 0 0 false "ECC_Visibility")
                  ;[1 1 1] Sound
                  (Audio|PlaySoundatLocation "/Game/PrototypeWeap/Sound/GrenadeLauncher/GL_Explosion04.GL_Explosion04" (Transformation|GetWorldLocation (Variables|Default|GetCube)) "0, 0, 0" (Variables|RedColorEffect|GetDamageSound) 1.0 0.0 0 0 0))))))
        (:1
          (Utilities|FlowControl|Sequence
            (:then_0
              (if (not (>= (Variables|Default|GetCountB) 1.0))
                (bind _output_get_2 (Variables|Default|SetCountB (+ (Variables|Default|GetCountB) 0.1)))
                (Rendering|Material|SetVectorParameterValue (Variables|Default|GetDynamic%20Material) "BaseColor" (Math|Color|MakeColor 0.0 0.0 _output_get_2) :!class /Script/Engine.MaterialInstanceDynamic)))
            (:then_1
              (Rendering|SetVisibility _p_fire false false)
              (Rendering|SetVisibility _p_sparks true false)
              (Actor|DestroyActor (Variables|Default|GetProj))
              (if (Variables|ColorEffectsVar|GetActivBlueEffect)
                ;[1 1 1] Blue Color Effect | Spawns BlueColorSphere -> Effect is there (BlueColorSphere BP)
                (if (>= (Variables|Default|GetCountB) 1.0)
                  (Utilities|FlowControl|DoOnce false
                    (:Completed
                      (bind _returnvalue (Game|SpawnActorfromClass "/Game/Blueprints/ColorEffectBlocks/BlueColorSphere.BlueColorSphere_C" (Math|Transform|MakeTransform (Transformation|GetWorldLocation _cube_3) (Transformation|GetWorldRotation _cube_3) (Math|Conversions|ToVector(Float) (/ (Variables|BlueColorEffect|GetBlueRadius) 5e+01))) "AlwaysSpawn" 0 0))
                      (Utilities|FlowControl|Sequence
                        (:then_0
                          (Audio|PlaySoundatLocation "/Engine/EditorSounds/GamePreview/PossessPlayer.PossessPlayer" (Transformation|GetWorldLocation (Variables|Default|GetCube)) "0, 0, 0" 0.5 1.0 0.0 0 0 0))
                        (:then_1
                          (Utilities|FlowControl|Delay (Variables|BlueColorEffect|GetBlueEffectTime))
                          (if (Utilities|IsValid _returnvalue)
                            (Actor|DestroyActor _returnvalue)))))))))))
        (:2
          (Utilities|FlowControl|Sequence
            (:then_0
              (if (not (>= (Variables|Default|GetCountG) 1.0))
                (bind _output_get_3 (Variables|Default|SetCountG (+ (Variables|Default|GetCountG) 0.1)))
                (Rendering|Material|SetVectorParameterValue (Variables|Default|GetDynamic%20Material) "BaseColor" (Math|Color|MakeColor 0.0 _output_get_3 0.0) :!class /Script/Engine.MaterialInstanceDynamic)))
            (:then_1
              (Rendering|SetVisibility _p_fire false false)
              (Rendering|SetVisibility _p_sparks false false)
              (Actor|DestroyActor (Variables|Default|GetProj))
              (if (Variables|ColorEffectsVar|GetActivGreenEffect)
                ;[1 1 1] Green Color Effect | 0: Repair near destroyed Blocks(+Reset) | 1: Heal Player | 2: Create new Blocks
                (if (>= (Variables|Default|GetCountG) 1.0)
                  (Utilities|FlowControl|Sequence
                    (:then_0
                      (if (Variables|GreenColorEffect|GetRestoreBlocks)
                        (bind _outactors (Actor|GetAllActorsOfClass "ColorEffect_Parent_C"))
                        (for _array_element _outactors
                          (if (<= (Math|Vector|VectorLength (- (Transformation|GetWorldLocation (Variables|ColorEffect_Parent_C|GetCube _array_element)) (Transformation|GetWorldLocation (Variables|Default|GetCube)))) (Variables|GreenColorEffect|GetBlockHealingRadius))
                            (if (not (Variables|/Script/Engine.SceneComponent|GetbVisible (Variables|ColorEffect_Parent_C|GetCube _array_element)))
                              (Rendering|Material|SetVectorParameterValue (Variables|ColorEffect_Parent_C|GetDynamic%20Material _array_element) "BaseColor" (Math|Color|MakeColor 0.0 0.0 0.0) :!class /Script/Engine.MaterialInstanceDynamic)
                              (Variables|ColorEffect_Parent_C|SetCountR _array_element 0.1)
                              (Variables|ColorEffect_Parent_C|SetCountB _array_element 0.1)
                              (Variables|ColorEffect_Parent_C|SetCountR _array_element 0.1)
                              (Rendering|SetVisibility (Variables|ColorEffect_Parent_C|GetCube _array_element) true false)
                              (Collision|SetCollisionEnabled (Variables|ColorEffect_Parent_C|GetCube _array_element) "QueryAndPhysics")
                              (Rendering|SetVisibility (Variables|Default|GetP_Fire) true false)
                              ;[1 1 1] Play Sound
                              (Audio|PlaySoundatLocation "/Game/Sounds/GreenColorBlock.GreenColorBlock" (Transformation|GetWorldLocation (Variables|Default|GetCube)) "0, 0, 0" 0.3 1.0 0.0 0 0 0))))))
                    (:then_1
                      (if (Variables|GreenColorEffect|GetActivatePlayerHealing)
                        (bind _asfirst_person_character (Utilities|Casting|CastToFirstPersonCharacter (Game|GetPlayerCharacter 0)))
                        (Variables|/Game/PlayerBP/Blueprints/FirstPersonCharacter.FirstPersonCharacter_C|SetCurrHealth _asfirst_person_character (+ (Variables|GreenColorEffect|GetPlayerHealing) (Variables|/Game/PlayerBP/Blueprints/FirstPersonCharacter.FirstPersonCharacter_C|GetCurrHealth _asfirst_person_character)))
                        (Variables|GreenColorEffect|SetActivatePlayerHealing false)))
                    (:then_2
                      (if (Variables|GreenColorEffect|GetTornado)
                        (Utilities|FlowControl|DoOnce false
                          (:Completed
                            (for _index (range 0 2)
                              (Game|SpawnActorfromClass "/Game/Blueprints/ColorEffectBlocks/GreenEffect.GreenEffect_C" (Math|Transform|MakeTransform (Transformation|GetWorldLocation _cube_2) (Transformation|GetWorldRotation _cube_2)) "Undefined" 0 (Variables|GreenColorEffect|GetTornado_Red) (Variables|GreenColorEffect|GetTornado_Blue) (Variables|GreenColorEffect|GetTornado_Green) 0))))))))))))
        (:3
          ;[1 1 1] Enemy Shoot (Paint Black, Reset Color)
          (Rendering|Material|SetVectorParameterValue (Variables|Default|GetDynamic%20Material) "BaseColor" "(R=0.008000,G=0.008000,B=0.008000,A=1.000000)" :!class /Script/Engine.MaterialInstanceDynamic)
          (Rendering|SetVisibility (Variables|Default|GetP_Fire) false false)
          (Variables|Default|SetCountR 0.1)
          (Variables|Default|SetCountB 0.1)
          (Variables|Default|SetCountG 0.1)
          (Actor|DestroyActor (Variables|Default|GetProj))
          (Variables|Default|SetBlackCooldown true)
          (Utilities|FlowControl|Delay (Variables|ColorEffectsVar|GetBlackColorCooldown))
          (Variables|Default|SetBlackCooldown false))))))

(event OnComponentBeginOverlap(SphereCollision)
  (params (OverlappedComponent :type Primitive%20Component%20Object%20Reference) (OtherActor :type Actor%20Object%20Reference) (OtherComp :type Primitive%20Component%20Object%20Reference) (OtherBodyIndex :type Integer) (bFromSweep :type Boolean) (SweepResult :type Hit%20Result%20Structure%20%28by%20ref%29))
  ;[1 1 1] Check is Player in Range
  (bind _asfirst_person_character (Utilities|Casting|CastToFirstPersonCharacter OtherActor))
  (Variables|Default|SetPlayerinRange true)
  (if (Variables|Default|GetHasColor)
    (Default|ColorBlockNear _asfirst_person_character (Variables|ColorEffectsVar|GetBlockValue) 0.0)
    (else
      (Default|ColorBlockNear _asfirst_person_character 0.0 (Variables|ColorEffectsVar|GetBlockValue)))))

(event OnComponentEndOverlap(SphereCollision)
  (params (OverlappedComponent :type Primitive%20Component%20Object%20Reference) (OtherActor :type Actor%20Object%20Reference) (OtherComp :type Primitive%20Component%20Object%20Reference) (OtherBodyIndex :type Integer))
  ;[1 1 1] Check is Player in Range
  (bind _asfirst_person_character (Utilities|Casting|CastToFirstPersonCharacter OtherActor))
  (Variables|Default|SetPlayerinRange false)
  (if (Variables|Default|GetHasColor)
    (Default|ColorBlockNear _asfirst_person_character (* (Variables|ColorEffectsVar|GetBlockValue) -1.0) 0.0)
    (else
      (Default|ColorBlockNear _asfirst_person_character 0.0 (* (Variables|ColorEffectsVar|GetBlockValue) -1.0)))))

(event Custom|Update%20Change%20HasColor
  (bind _blockvalue (Variables|ColorEffectsVar|GetBlockValue))
  (bind _blockvalue_2 (Variables|ColorEffectsVar|GetBlockValue))
  ;[1 1 1] On Block Change Color
  (if (not (Math|Boolean|Equal(Boolean) (Variables|Default|GetHasColor) (Variables|Default|GetHasColorChange)))
    (Variables|Default|SetHasColorChange (Variables|Default|GetHasColor))
    (if (Variables|Default|GetPlayerinRange)
      (bind _asfirst_person_character (Utilities|Casting|CastToFirstPersonCharacter (Game|GetPlayerCharacter 0)))
      (if (Variables|Default|GetHasColor)
        (Default|ColorBlockNear _asfirst_person_character _blockvalue (* _blockvalue -1.0))
        (else
          (Default|ColorBlockNear _asfirst_person_character (* _blockvalue_2 -1.0) _blockvalue_2))))))

(event Custom|Update%20Color
  (bind _sphere (Variables|Default|GetSphere))
  ;[1 1 1] Check has Block currently Color? Dark Sphere Yes/No
  (if (== (Variables|/Game/PlayerBP/Blueprints/ColorEffectProjectile.ColorEffectProjectile_C|GetColorVal (stale OnComponentBeginOverlap(Cube) _ascolor_effect_projectile)) 3)
    (Variables|Default|SetHasColor false)
    (Rendering|SetVisibility _sphere true false)
    (else
      (Variables|Default|SetHasColor true)
      (Rendering|SetVisibility _sphere false false)))
  (CallFunction|UpdateChangeHasColor))

(event EventBeginPlay
  ;[1 1 1] Detection Radius
  (Transformation|SetWorldScale3D (Variables|Default|GetSphereCollision) "30.000000,30.000000,30.000000")
  (Rendering|Material|SetVectorParameterValue (Variables|Default|GetDynamic%20Material) "BaseColor" "(R=0.008000,G=0.008000,B=0.008000,A=1.000000)" :!class /Script/Engine.MaterialInstanceDynamic))

(fn ConstructionScript
  (bind _sphere (Variables|Default|GetSphere))
  (bind _cube (Variables|Default|GetCube))
  ;[1 1 1] Make Cube Material possible to change Color
  (bind _returnvalue (Rendering|Material|CreateDynamicMaterialInstance (Variables|Default|GetCube) 0 0 "None" :!class /Script/Engine.PrimitiveComponent))
  (Variables|Default|SetDynamic%20Material _returnvalue)
  ;[1 1 1] Start Visible?
  (if (Variables|Visual|GetstartVisible)
    (Rendering|SetVisibility _cube true false)
    (Collision|SetCollisionEnabled (Variables|Default|GetCube) "QueryAndPhysics")
    (else
      (Rendering|SetVisibility _cube false false)
      (Collision|SetCollisionEnabled (Variables|Default|GetCube) "NoCollision")
      (Rendering|SetVisibility (Variables|Default|GetP_Fire) false false)))
  ;[1 1 1] Show Black Sphere
  (if (Variables|Visual|GetshowBlackSphere)
    (Rendering|SetVisibility _sphere true false)
    (else
      (Rendering|SetVisibility _sphere false false)))
  ;[1 1 1] Enable/Disable Icon
  (Rendering|Material|SetTextureParameterValue (Variables|Default|GetDynamic%20Material) "Icon" (Variables|Visual|GetIcon)))