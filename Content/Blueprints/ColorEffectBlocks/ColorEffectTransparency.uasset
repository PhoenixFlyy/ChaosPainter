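; A block that starts see-through or opaque by a material Transparency_Amount and changes color when hit by ColorEffectProjectiles.
; Each overlap raises that projectile's red, blue or green counter, sets BaseColor to that channel alone, and bumps the transparency value on a dynamic material instance.
; Enough red hides the cube, disables its collision and plays an explosion.
; While ReColor is set, a delayed Tick gradually lowers the transparency value back down.
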(event EventTick
  (params (DeltaSeconds :type Float%20%28single-precision%29))
  ;[1 1 1] Make it slowly back Transparent
  (if (Variables|ColorEffectsVar|GetReColor)
    (Utilities|FlowControl|Delay 0.1)
    (if (> (Variables|Default|GetCountV) 0.0)
      (bind _output_get (Variables|Default|SetCountV (- (Variables|Default|GetCountV) 0.01)))
      (Rendering|Material|SetScalarParameterValue (Variables|Default|GetDynamic%20Material) "Transparency_Amount" _output_get :!class /Script/Engine.MaterialInstanceDynamic))))

(event Collision|EventActorBeginOverlap
  (params (OtherActor :type Actor%20Object%20Reference))
  (bind _cube (Variables|Default|GetCube))
  (bind _dynamic_material (Variables|Default|GetDynamic%20Material))
  ;[1 1 1] Projectile Overlap Event | Get Projectile Color
  (bind _ascolor_effect_projectile (Utilities|Casting|CastToColorEffectProjectile OtherActor))
  (switch int (Variables|/Game/PlayerBP/Blueprints/ColorEffectProjectile.ColorEffectProjectile_C|GetColorVal _ascolor_effect_projectile)
    (:0
      ;[1 1 1] Counting Collisions (Adding Color)
      (bind _output_get (Variables|Default|SetCountR (+ (Variables|Default|GetCountR) 0.1)))
      ;[1 1 1] Graphic Visibility
      (Rendering|Material|SetVectorParameterValue _dynamic_material "BaseColor" (Math|Color|MakeColor _output_get 0.0 0.0) :!class /Script/Engine.MaterialInstanceDynamic))
    (:1
      (bind _output_get_2 (Variables|Default|SetCountB (+ (Variables|Default|GetCountB) 0.1)))
      (Rendering|Material|SetVectorParameterValue _dynamic_material "BaseColor" (Math|Color|MakeColor 0.0 0.0 _output_get_2) :!class /Script/Engine.MaterialInstanceDynamic))
    (:2
      (bind _output_get_3 (Variables|Default|SetCountG (+ (Variables|Default|GetCountG) 0.1)))
      (Rendering|Material|SetVectorParameterValue _dynamic_material "BaseColor" (Math|Color|MakeColor 0.0 _output_get_3 0.0) :!class /Script/Engine.MaterialInstanceDynamic)))
  ;[1 1 1] Set Transparency | Destroy Block if to much Red Color applied
  (if (>= (Variables|Default|GetCountV) 1.05)
    _
    (else
      (bind _output_get_4 (Variables|Default|SetCountV (+ (Variables|Default|GetCountV) 0.05)))))
  (Rendering|Material|SetScalarParameterValue (Variables|Default|GetDynamic%20Material) "Transparency_Amount" _output_get_4 :!class /Script/Engine.MaterialInstanceDynamic)
  (if (>= (Variables|Default|GetCountR) 1.0)
    (Rendering|SetVisibility _cube false false)
    (Collision|SetCollisionEnabled _cube "NoCollision")
    ;[1 1 1] Sound
    (Audio|PlaySoundatLocation "/Game/PrototypeWeap/Sound/GrenadeLauncher/GL_Explosion04.GL_Explosion04" (Transformation|GetWorldLocation (Variables|Default|GetCube)) "0, 0, 0" 0.3 1.0 0.0 0 0 0)))

(fn ConstructionScript
  ;[1 1 1] Make Cube Material possible to change Color
  (bind _returnvalue (Rendering|Material|CreateDynamicMaterialInstance (Variables|Default|GetCube) 0 0 "None" :!class /Script/Engine.PrimitiveComponent))
  (Variables|Default|SetDynamic%20Material _returnvalue))