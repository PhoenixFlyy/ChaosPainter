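; A turbine color-effect block that spins its Cube under the green effect and extends its red effect to four extra parts.
; While green is active and its count reaches one, Tick replays a rotation timeline on the pitch from the starting rotation, doubled when Turbo is on.
; Tick also mirrors the Cube's visibility onto the four parts and their collision, using DoOnce gates with short delays to switch only on changes.
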(event EventTick
  (params (DeltaSeconds :type Float%20%28single-precision%29))
  (bind _self self)
  (bind _baserotation (Variables|Default|GetBaseRotation))
  (bind _baserotation_2 (Variables|Default|GetBaseRotation))
  (bind _2 (Variables|Default|Get2))
  (bind _2_2 (Variables|Default|Get2))
  (bind (_roll _pitch _yaw) (Math|Rotator|BreakRotator _baserotation_2))
  (bind (_roll_2 _pitch_2 _yaw_2) (Math|Rotator|BreakRotator _baserotation))
  (Utilities|FlowControl|Sequence
    (:then_0
      ;[1 1 1] Create Rotation
      (if (Variables|Default|GetActivGreenEffect _self)
        (if (>= (Variables|Default|GetCountG _self) 1.0)
          (Utilities|FlowControl|DoOnce false :!label _label
            (:Completed
              (bind _rotation (Timeline|RotationTimeline PlayFromStart)
                (:Update
                  (if (Variables|Default|GetTurbo)
                    (Transformation|SetWorldRotation (Variables|Default|GetCube) (Math|Rotator|MakeRotator _roll (* _rotation 2.0) _yaw) false false)
                    (else
                      (Transformation|SetWorldRotation (Variables|Default|GetCube) (Math|Rotator|MakeRotator _roll_2 _rotation _yaw_2) false false))))
                (:Finished
                  (goto _label Reset))))))
        (else
          (goto _label))))
    (:then_1
      ;[1 1 1] Red Color Effect Extension
      (if (Rendering|IsVisible (Variables|Default|GetCube))
        (Utilities|FlowControl|DoOnce true :!label _label_2
          (:Completed
            (Rendering|SetVisibility _2 true false)
            (Collision|SetCollisionEnabled _2 "QueryAndPhysics")
            (Utilities|FlowControl|Delay 0.2)
            (goto _label_3 Reset)))
        (else
          (Utilities|FlowControl|DoOnce false :!label _label_3
            (:Completed
              (Rendering|SetVisibility _2_2 false false)
              (Collision|SetCollisionEnabled _2_2 "NoCollision")
              (Utilities|FlowControl|Delay 0.2)
              (goto _label_2 Reset))))))))

(event EventBeginPlay
  ;[1 1 1] Get Base Rotation at Start
  (|CallParentFunction)
  (Variables|Default|SetBaseRotation (Transformation|GetWorldRotation (Variables|Default|GetCube))))

(fn ConstructionScript
  (|CallParentFunction))