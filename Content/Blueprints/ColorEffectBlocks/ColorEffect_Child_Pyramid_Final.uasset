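; Child color-effect block for a final pyramid that sinks while rotating when red is applied, then triggers an ending cinematic.
; Tick detects the hidden Cube, re-shows it once and runs the Fall timeline to offset its height and yaw.
; When that finishes, FirstPersonCharacter's Final counter selects one of four level sequences, played with input, player and HUD disabled or hidden.
; The counter then increments and the Cube hides again.
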(event EventTick
  (params (DeltaSeconds :type Float%20%28single-precision%29))
  (bind _moviescenesequenceplaybacksettings (Utilities|Struct|MakeMovieSceneSequencePlaybackSettings false "(Value=0)" 1.0 0.0 false false true false true true))
  (bind _cube (Variables|Default|GetCube))
  ;[1 1 1] When Red Color Applied -> Rotation Down
  (if (not (Rendering|IsVisible (Variables|Default|GetCube)))
    (Utilities|FlowControl|DoOnce false
      (:Completed
        (Variables|Default|SetBaseLocation (Transformation|GetWorldLocation _cube))
        (Variables|Default|SetBaseRotation (Transformation|GetWorldRotation _cube))
        (Rendering|SetVisibility (Variables|Default|GetCube) true false)
        (bind (_direction _location_z _rotation_z) (Timeline|Fall PlayFromStart)
          (:Update
            (Transformation|SetWorldLocationAndRotation (Variables|Default|GetCube) (Math|Vector|MakeVector (.X (Math|Vector|BreakVector (Variables|Default|GetBaseLocation))) (.Y (Math|Vector|BreakVector (Variables|Default|GetBaseLocation))) (- (.Z (Math|Vector|BreakVector (Variables|Default|GetBaseLocation))) _location_z)) (Math|Rotator|MakeRotator (.Roll (Math|Rotator|BreakRotator (Variables|Default|GetBaseRotation))) (.Pitch (Math|Rotator|BreakRotator (Variables|Default|GetBaseRotation))) (+ _rotation_z (.Yaw (Math|Rotator|BreakRotator (Variables|Default|GetBaseRotation))))) false false))
          (:Finished
            ;[1 1 1] Play Final Sequence
            (Utilities|FlowControl|DoOnce false
              (:Completed
                (Utilities|FlowControl|Sequence
                  (:then_0
                    (bind _asfirst_person_character (Utilities|Casting|CastToFirstPersonCharacter (Game|GetPlayerCharacter 0)))
                    (switch int (Variables|/Game/PlayerBP/Blueprints/FirstPersonCharacter.FirstPersonCharacter_C|GetFinal _asfirst_person_character)
                      (:0
                        (bind _returnvalue (Sequencer|Player|CreateLevelSequencePlayer "/Game/Cinematic/Final_1.Final_1" _moviescenesequenceplaybacksettings))
                        (Sequencer|Player|Play _returnvalue :!class /Script/MovieScene.MovieSceneSequencePlayer))
                      (:1
                        (bind _returnvalue_2 (Sequencer|Player|CreateLevelSequencePlayer "/Game/Cinematic/Final_2.Final_2" _moviescenesequenceplaybacksettings))
                        (Sequencer|Player|Play _returnvalue_2 :!class /Script/MovieScene.MovieSceneSequencePlayer))
                      (:2
                        (bind _returnvalue_3 (Sequencer|Player|CreateLevelSequencePlayer "/Game/Cinematic/Final_3.Final_3" _moviescenesequenceplaybacksettings))
                        (Sequencer|Player|Play _returnvalue_3 :!class /Script/MovieScene.MovieSceneSequencePlayer))
                      (:3
                        (bind _returnvalue_4 (Sequencer|Player|CreateLevelSequencePlayer "/Game/Cinematic/Final_4.Final_4" _moviescenesequenceplaybacksettings))
                        (Sequencer|Player|Play _returnvalue_4 :!class /Script/MovieScene.MovieSceneSequencePlayer)))
                    (Variables|/Game/PlayerBP/Blueprints/FirstPersonCharacter.FirstPersonCharacter_C|SetFinal _asfirst_person_character (+ (Variables|/Game/PlayerBP/Blueprints/FirstPersonCharacter.FirstPersonCharacter_C|GetFinal _asfirst_person_character) 1)))
                  (:then_1
                    (Rendering|SetVisibility (Variables|Default|GetCube) false false)))))))))))

(fn ConstructionScript
  (|CallParentFunction))