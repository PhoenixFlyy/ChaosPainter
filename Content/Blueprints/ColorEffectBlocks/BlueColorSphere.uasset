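; Blue color effect sphere that boosts the first-person character's walk speed and jump height while the player is inside it.
; The sphere mesh becomes visible shortly after spawn, timed to a lightning hit.
; Overlap begin flags the player as inside, raises movement values and adds a BlueSphereEffect screen widget.
; Leaving or EndPlay restores walk or sprint speed and jump velocity and removes the widget; only leaving clears the flag.
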(event EventBeginPlay
  ;[1 1 1] Sphere Visible when Lightning hits
  (Utilities|FlowControl|Delay 0.3)
  (Rendering|SetVisibility (Variables|Default|GetSphere) true false))

(event Collision|EventActorBeginOverlap
  (params (OtherActor :type Actor%20Object%20Reference))
  ;[1 1 1] Check is Player in Sphere | BlueColorEffect
  (bind _asfirst_person_character (Utilities|Casting|CastToFirstPersonCharacter OtherActor))
  (Variables|/Game/PlayerBP/Blueprints/FirstPersonCharacter.FirstPersonCharacter_C|SetIsInBlueSphere _asfirst_person_character true)
  (Variables|/Script/Engine.CharacterMovementComponent|SetMaxWalkSpeed (Variables|/Script/Engine.Character|GetCharacterMovement _asfirst_person_character) 1.2e+03)
  (Variables|/Script/Engine.CharacterMovementComponent|SetJumpZVelocity (Variables|/Script/Engine.Character|GetCharacterMovement _asfirst_person_character) 7.5e+02)
  (bind _returnvalue (UserInterface|CreateWidget "/Game/PlayerBP/Widgets/BlueSphereEffect.BlueSphereEffect_C" (Game|GetPlayerController 0)))
  (Variables|Default|SetBlueSphereWid _returnvalue)
  (UserInterface|Viewport|AddtoViewport (Variables|Default|GetBlueSphereWid) 0))

(event Collision|EventActorEndOverlap
  (params (OtherActor :type Actor%20Object%20Reference))
  ;[1 1 1] Is Player not in Sphere or Event End | Remove BlueColorEffects
  (bind _asfirst_person_character (Utilities|Casting|CastToFirstPersonCharacter OtherActor))
  (Variables|/Game/PlayerBP/Blueprints/FirstPersonCharacter.FirstPersonCharacter_C|SetIsInBlueSphere _asfirst_person_character false)
  (if (Variables|/Game/PlayerBP/Blueprints/FirstPersonCharacter.FirstPersonCharacter_C|GetSprintKey _asfirst_person_character)
    (Variables|/Script/Engine.CharacterMovementComponent|SetMaxWalkSpeed (Variables|/Script/Engine.Character|GetCharacterMovement _asfirst_person_character) 8.5e+02)
    (else
      (Variables|/Script/Engine.CharacterMovementComponent|SetMaxWalkSpeed (Variables|/Script/Engine.Character|GetCharacterMovement _asfirst_person_character) 6e+02)))
  (Variables|/Script/Engine.CharacterMovementComponent|SetJumpZVelocity (Variables|/Script/Engine.Character|GetCharacterMovement _asfirst_person_character) 5e+02)
  (Widget|RemovefromParent (Variables|Default|GetBlueSphereWid)))

(event EventEndPlay
  (params (EndPlayReason :type EEndPlayReason%20Enum :default "Destroyed"))
  ;[1 1 1] Is Player not in Sphere or Event End | Remove BlueColorEffects
  (bind _asfirst_person_character (Utilities|Casting|CastToFirstPersonCharacter (Game|GetPlayerCharacter 0)))
  (if (Variables|/Game/PlayerBP/Blueprints/FirstPersonCharacter.FirstPersonCharacter_C|GetSprintKey _asfirst_person_character)
    (Variables|/Script/Engine.CharacterMovementComponent|SetMaxWalkSpeed (Variables|/Script/Engine.Character|GetCharacterMovement _asfirst_person_character) 8.5e+02)
    (else
      (Variables|/Script/Engine.CharacterMovementComponent|SetMaxWalkSpeed (Variables|/Script/Engine.Character|GetCharacterMovement _asfirst_person_character) 6e+02)))
  (Variables|/Script/Engine.CharacterMovementComponent|SetJumpZVelocity (Variables|/Script/Engine.Character|GetCharacterMovement _asfirst_person_character) 5e+02)
  (Widget|RemovefromParent (Variables|Default|GetBlueSphereWid)))

(fn ConstructionScript)