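; BP_Intro plays the game's intro cinematic when play begins, provided the player character is a FirstPersonCharacter.
; A DoOnce gate starts three level sequences in order: StoryIntro, Intro1 and StoryIntro2.
; Each gets its own sequence player that disables movement input and hides the player and HUD.
; Fixed delays space the sequences, with no binding to their finish events.
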(event EventBeginPlay
  (bind _moviescenesequenceplaybacksettings (Utilities|Struct|MakeMovieSceneSequencePlaybackSettings false "(Value=0)" 1.0 0.0 false false true false true true))
  (Utilities|Casting|CastToFirstPersonCharacter (Game|GetPlayerCharacter 0))
  (Utilities|FlowControl|DoOnce false
    (:Completed
      (bind _returnvalue (Sequencer|Player|CreateLevelSequencePlayer "/Game/Cinematic/StoryIntro.StoryIntro" _moviescenesequenceplaybacksettings))
      (Sequencer|Player|Play _returnvalue :!class /Script/MovieScene.MovieSceneSequencePlayer)
      (Utilities|FlowControl|Delay 5.0)
      (bind _returnvalue_2 (Sequencer|Player|CreateLevelSequencePlayer "/Game/Cinematic/Intro1.Intro1" _moviescenesequenceplaybacksettings))
      (Sequencer|Player|Play _returnvalue_2 :!class /Script/MovieScene.MovieSceneSequencePlayer)
      (Utilities|FlowControl|Delay 5.0)
      (bind _returnvalue_3 (Sequencer|Player|CreateLevelSequencePlayer "/Game/Cinematic/StoryIntro2.StoryIntro2" _moviescenesequenceplaybacksettings))
      (Sequencer|Player|Play _returnvalue_3 :!class /Script/MovieScene.MovieSceneSequencePlayer))))

(fn ConstructionScript)