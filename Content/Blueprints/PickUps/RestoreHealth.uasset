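; RestoreHealth is a pickup that gradually refills the first-person character's health while they stay inside its capsule.
; The first overlap computes one fortieth of the missing health and starts a one-shot Refill timeline, which adds that amount on each update while the player is in range.
; Leaving the capsule pauses healing but not the timeline, and the actor destroys itself when the timeline finishes.
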(event OnComponentBeginOverlap(Capsule)
  (params (OverlappedComponent :type Primitive%20Component%20Object%20Reference) (OtherActor :type Actor%20Object%20Reference) (OtherComp :type Primitive%20Component%20Object%20Reference) (OtherBodyIndex :type Integer) (bFromSweep :type Boolean) (SweepResult :type Hit%20Result%20Structure%20%28by%20ref%29))
  (bind _asfirst_person_character (Utilities|Casting|CastToFirstPersonCharacter OtherActor))
  (Variables|Default|SetPlayerInstance _asfirst_person_character)
  (Variables|Default|SetPlayerInRange true)
  (Utilities|FlowControl|DoOnce false
    (:Completed
      (Variables|Default|SetCount (/ (- (Variables|/Game/PlayerBP/Blueprints/FirstPersonCharacter.FirstPersonCharacter_C|GetMaxHealth (Variables|Default|GetPlayerInstance)) (Variables|/Game/PlayerBP/Blueprints/FirstPersonCharacter.FirstPersonCharacter_C|GetCurrHealth (Variables|Default|GetPlayerInstance))) 4e+01))
      (Timeline|Refill_Timeline Play
        (:Finished
          (Actor|DestroyActor))
        (:Exec%20Update
          (if (Variables|Default|GetPlayerInRange)
            (Variables|/Game/PlayerBP/Blueprints/FirstPersonCharacter.FirstPersonCharacter_C|SetCurrHealth (Variables|Default|GetPlayerInstance) (+ (Variables|/Game/PlayerBP/Blueprints/FirstPersonCharacter.FirstPersonCharacter_C|GetCurrHealth (Variables|Default|GetPlayerInstance)) (Variables|Default|GetCount)))))))))

(event OnComponentEndOverlap(Capsule)
  (params (OverlappedComponent :type Primitive%20Component%20Object%20Reference) (OtherActor :type Actor%20Object%20Reference) (OtherComp :type Primitive%20Component%20Object%20Reference) (OtherBodyIndex :type Integer))
  (Utilities|Casting|CastToFirstPersonCharacter OtherActor)
  (Variables|Default|SetPlayerInRange false))

(fn ConstructionScript)