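; FloatingText is an actor that shows world-space text when the player character is within range.
; The construction script applies the TextVal and TextColor variables to its TextRender component.
; Each tick, it compares the player's distance to ActiveRange, shows or hides the text, and rotates visible text to face the player character's location rather than the camera.
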(event EventTick
  (params (DeltaSeconds :type Float%20%28single-precision%29))
  (bind _textrender (Variables|Default|GetTextRender))
  (if (<= (Math|Vector|VectorLength (- (Transformation|GetActorLocation (Game|GetPlayerCharacter 0)) (Transformation|GetActorLocation))) (Variables|Default|GetActiveRange))
    (Rendering|SetVisibility _textrender true false)
    (Transformation|SetWorldRotation (Variables|Default|GetTextRender) (Math|Rotator|FindLookatRotation (Transformation|GetActorLocation) (Transformation|GetActorLocation (Game|GetPlayerCharacter 0))) false false)
    (else
      (Rendering|SetVisibility _textrender false false))))

(fn ConstructionScript
  (Rendering|Components|TextRender|SetText (Variables|Default|GetTextRender) (Variables|Default|GetTextVal))
  (Rendering|Components|TextRender|SetTextRenderColor (Variables|Default|GetTextRender) (Math|Conversions|ToColor(LinearColor) (Variables|Default|GetTextColor))))